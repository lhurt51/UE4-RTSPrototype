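; RTS GameState that runs the in-game clock and calendar.
; Tick advances GameTime in hours at GameSpeed, derives clock and date with month and year rollover, pushes both to the player controller's HUD, and prints the date.
; UpdateGameSpeed writes the scaled default speed into GameTime, not GameSpeed, and passes it to GameSpeedControl.
; SetGameCalendar and SetGameClock are stubs returning false.
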(event EventBeginPlay
  (Utilities|FlowControl|Sequence
    (:then_0
      (Utilities|ReferenceCast))
    (:then_1
      (Variables|GameTimeSettings|SetGameTime (+ (Math|Conversions|ToFloat(Integer) (Variables|Clock|GetHours)) (/ (Math|Conversions|ToFloat(Integer) (Variables|Clock|GetMinutes)) 6e+01) (/ (Math|Conversions|ToFloat(Integer) (Variables|Clock|GetSeconds)) 3.6e+03))))
    (:then_2
      (Variables|GameTimeSettings|SetGameSpeed (Variables|GameTimeSettings|GetDefaultGameSpeed)))))

(event EventTick
  (params (DeltaSeconds :type Float%20%28single-precision%29))
  (Variables|GameTimeSettings|SetGameTime (.GameTime (CallFunction|SetGameTime DeltaSeconds (Variables|GameTimeSettings|GetGameSpeed) (Variables|GameTimeSettings|GetGameTime))))
  (Variables|Calendar|SetDayCounter (.DayCount (CallFunction|SetGameTime DeltaSeconds (Variables|GameTimeSettings|GetGameSpeed) (Variables|GameTimeSettings|GetGameTime))))
  (Clock|SetClock)
  (Calendar|SetCalendar)
  (bind _output_get (Variables|Default|SetGameDate (Math|DateTime|MakeDateTime (Variables|Calendar|GetYear) (Variables|Calendar|GetMonth) (Variables|Calendar|GetDay) (Variables|Clock|GetHours) (Variables|Clock|GetMinutes) (Variables|Clock|GetSeconds))))
  (Development|PrintString (Utilities|String|ToString(Text) (Class|KismetTextLibrary|AsTimeZoneDateTimeDateTime _output_get "UTC"))))

(event EventUpdateGameSpeed
  (params (SpeedMultiplier :type Float%20%28single-precision%29))
  (bind _output_get (Variables|GameTimeSettings|SetSpeedMultiplier SpeedMultiplier))
  (Variables|GameTimeSettings|SetGameTime (* _output_get (Variables|GameTimeSettings|GetDefaultGameSpeed)))
  (Default|CallGameSpeedControl (Variables|GameTimeSettings|GetGameTime)))

(fn ConstructionScript)

(fn SetClock
  (bind _gametime (Variables|GameTimeSettings|GetGameTime))
  (bind _returnvalue (* _gametime 3.6e+03))
  (bind (_remainder _returnvalue_2) (Math|Float|Division(WholeandRemainder) _returnvalue 6e+01))
  (bind _returnvalue_3 (Math|Conversions|ToFloat(Integer) _returnvalue_2))
  (bind (_remainder_2 _returnvalue_4) (Math|Float|Division(WholeandRemainder) _returnvalue_3 6e+01))
  (Variables|Clock|SetSeconds (Math|Float|Floor _remainder))
  (Variables|Clock|SetMinutes (Math|Float|Floor _remainder_2))
  (Variables|Clock|SetHours (Math|Float|Floor (.Remainder (Math|Float|Division(WholeandRemainder) (Math|Conversions|ToFloat(Integer) _returnvalue_4) 24.0))))
  (Class|BPGameTimeIRTS|SetGameClock(Message) (Variables|/Game/RTS_Prototype/Blueprints/PlayableCamera/BP_PlayerController_RTS.BP_PlayerController_RTS_C|GetGameTimeHUDRef (Variables|References|GetControllerRef)) (Utilities|Array|MakeArray (Variables|Clock|GetSeconds) (Variables|Clock|GetMinutes) (Variables|Clock|GetHours))))

(fn SetCalendar
  (bind _output_get (Variables|Calendar|SetDay (+ (Variables|Calendar|GetDay) (Variables|Calendar|GetDayCounter))))
  (if (> _output_get (Class|KismetMathLibrary|DaysinMonth (Variables|Calendar|GetYear) (Variables|Calendar|GetMonth)))
    (Variables|Calendar|SetDay 1)
    (Variables|Calendar|SetMonth (+ (Variables|Calendar|GetMonth) 1)))
  (if (> (Variables|Calendar|GetMonth) 12)
    (Variables|Calendar|SetMonth 1)
    (Variables|Calendar|SetYear (+ (Variables|Calendar|GetYear) 1)))
  (Class|BPGameTimeIRTS|SetGameCalendar(Message) (Variables|/Game/RTS_Prototype/Blueprints/PlayableCamera/BP_PlayerController_RTS.BP_PlayerController_RTS_C|GetGameTimeHUDRef (Variables|References|GetControllerRef)) (Utilities|Array|MakeArray (Variables|Calendar|GetMonth) (Variables|Calendar|GetDay) (Variables|Calendar|GetYear))))

(fn GetGameSpeed
  (return (Variables|GameTimeSettings|GetGameSpeed)))

(fn SetGameCalendar
  (params (GameDate :type Array%20of%20Integers))
  (return false))

(fn SetGameClock
  (params (GameTime :type Array%20of%20Integers))
  (return false))