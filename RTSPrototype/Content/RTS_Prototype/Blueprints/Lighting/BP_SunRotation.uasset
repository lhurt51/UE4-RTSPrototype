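; BP_SunRotation rotates a referenced sun actor from game time to drive the sky's lighting, though a note marks it completely broken.
; BeginPlay caches BP_GameState_RTS, reads the starting game time and binds to game-speed control.
; Each Tick passes delta, speed and that time to SetGameTime, converts the result to pitch and adds it as local rotation.
; It then updates the sky sphere's sun direction.
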(event Custom|GetGameSpeed
  (params (GameSpeed :type Float%20%28single-precision%29))
  ;[1 1 1] Completely broken, need to fix this
  (Variables|Time|SetGameSpeed GameSpeed))

(event EventBeginPlay
  ;[1 1 1] Completely broken, need to fix this
  (Utilities|ReferenceCast)
  (EventDispatchers|BindEventtoGameSpeedControl (Variables|References|GetGameStateRef) (EventDispatchers|CreateEvent :!event Custom|GetGameSpeed))
  (bind _gametime (Default|GetGameTime (Variables|References|GetGameStateRef)))
  (Variables|Time|SetGameTime _gametime))

(event EventTick
  (params (DeltaSeconds :type Float%20%28single-precision%29))
  ;[1 1 1] Completely broken, need to fix this
  (Transformation|AddActorLocalRotation (Variables|References|GetSunRef) (Math|Rotator|MakeRotator 0.0 (* (/ (/ (.GameTime (CallFunction|SetGameTime DeltaSeconds (Variables|Time|GetGameSpeed) (Variables|Time|GetGameTime))) 1.5) 6.0) 9e+01) 0.0) false false)
  (Default|UpdateSunDirection (Variables|References|GetSkySphereRef)))

(fn ConstructionScript)