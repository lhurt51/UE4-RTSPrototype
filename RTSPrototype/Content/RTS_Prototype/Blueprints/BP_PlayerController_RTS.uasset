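; RTS player controller that drives the camera pawn, cast and cached on BeginPlay.
; Movement axes and screen-edge scrolling move the pawn relative to its facing via helper graphs, with a held speed modifier and key movement pinned to a fixed height.
; Zoom adjusts spring arm length within limits.
; Holding Pan opens gates that feed mouse input into yaw and clamped pitch while blocking movement; resets restore default zoom and level pitch.
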(event EventBeginPlay
  ;[1 1 1] Actor overrides
  (Utilities|FlowControl|Sequence
    (:then_0
      (Utilities|ReferenceCast))))

(event Input|ActionEvents|InputActionZoomReset
  (params (Key :type Key%20Structure :default "None"))
  ;[1 1 1] Camera Z Axis / Zoom Movement
  ;;[0.05415 0.8198 1] Reset spring arm length to default
  (:Pressed
    (Variables|/Script/Engine.SpringArmComponent|SetTargetArmLength (Variables|/Game/RTS_Prototype/Blueprints/BP_CameraPawn_RTS.BP_CameraPawn_RTS_C|GetSpringArm (Variables|References|GetCameraPawnRef)) 1.5e+03)))

(event Input|ActionEvents|InputActionZoomIn
  (params (Key :type Key%20Structure :default "None"))
  (bind _camerapawnref (Variables|References|GetCameraPawnRef))
  (bind _springarm (Variables|/Game/RTS_Prototype/Blueprints/BP_CameraPawn_RTS.BP_CameraPawn_RTS_C|GetSpringArm _camerapawnref))
  ;[1 1 1] Camera Z Axis / Zoom Movement
  ;;[1 0.1228 0.1825] Modifing the spring arm length to act as zoom
  (:Pressed
    (Variables|/Script/Engine.SpringArmComponent|SetTargetArmLength _springarm (Math|Float|Max(Float) (- (Variables|/Script/Engine.SpringArmComponent|GetTargetArmLength _springarm) (Variables|CameraMovement|GetZoomSpeed)) (Variables|CameraMovement|GetMinZoomLimit)))))

(event Input|ActionEvents|InputActionZoomOut
  (params (Key :type Key%20Structure :default "None"))
  (bind _camerapawnref (Variables|References|GetCameraPawnRef))
  (bind _springarm (Variables|/Game/RTS_Prototype/Blueprints/BP_CameraPawn_RTS.BP_CameraPawn_RTS_C|GetSpringArm _camerapawnref))
  ;[1 1 1] Camera Z Axis / Zoom Movement
  ;;[1 0.1228 0.1825] Modifing the spring arm length to act as zoom
  (:Pressed
    (Variables|/Script/Engine.SpringArmComponent|SetTargetArmLength _springarm (Math|Float|Min(Float) (+ (Variables|CameraMovement|GetZoomSpeed) (Variables|/Script/Engine.SpringArmComponent|GetTargetArmLength _springarm)) (Variables|CameraMovement|GetMaxZoomLimit)))))

(event Input|ActionEvents|InputActionPan
  (params (Key :type Key%20Structure :default "None"))
  (bind _camerapawnref (Variables|References|GetCameraPawnRef))
  (bind _returnvalue (Transformation|GetActorRotation _camerapawnref))
  ;[1 1 1] Camera Panning
  ;;[0 0.002892 1] Camera Pan X & Y
  (:Pressed
    (Variables|CameraMovement|SetDisableCameraMovement true)
    (Utilities|FlowControl|Gate true) ; enters at Open
  )
  (:Released
    (Variables|CameraMovement|SetDisableCameraMovement false)
    (Utilities|FlowControl|Gate true) ; enters at Close
  ))

(event Input|ActionEvents|InputActionPanReset
  (params (Key :type Key%20Structure :default "None"))
  (bind _camerapawnref (Variables|References|GetCameraPawnRef))
  (bind _returnvalue (Transformation|GetActorRotation _camerapawnref))
  ;[1 1 1] Camera Panning
  ;;[0 1 0.03342] Reset Camera Pan to Default
  (:Pressed
    (Transformation|SetActorRotation _camerapawnref (Math|Rotator|MakeRotator (.roll _returnvalue) 0.0 (.yaw _returnvalue)))))

(event Input|ActionEvents|InputActionPan
  (params (Key :type Key%20Structure :default "None"))
  (bind _camerapawnref (Variables|References|GetCameraPawnRef))
  (bind _returnvalue (Transformation|GetActorRotation _camerapawnref))
  ;[1 1 1] Camera Panning
  ;;[0 0.002892 1] Camera Pan X & Y
  (:Pressed
    (Variables|CameraMovement|SetDisableCameraMovement true)
    (Utilities|FlowControl|Gate true) ; enters at Open
  )
  (:Released
    (Variables|CameraMovement|SetDisableCameraMovement false)
    (Utilities|FlowControl|Gate true) ; enters at Close
  ))

(event Input|ActionEvents|InputActionSpeedModifier
  (params (Key :type Key%20Structure :default "None"))
  ;[1 1 1] Camera 2D Movement Controls
  ;;[1 0.03507 0.7658] Modify the camera movement speed
  (:Pressed
    (Variables|CameraMovement|SetMovementSpeedModifier 2.0))
  (:Released
    (Variables|CameraMovement|SetMovementSpeedModifier 1.0)))

(event Input|AxisEvents|InputAxisMoveForward
  (params (AxisValue :type Float%20%28single-precision%29))
  ;[1 1 1] Camera 2D Movement Controls
  ;;[0 0.9364 1] Camera 2D / X - Y Axis Movement
  (if (not (Variables|CameraMovement|GetDisableCameraMovement))
    (Utilities|BasicMovementControls AxisValue (stale Input|AxisEvents|InputAxisMoveRight AxisValue))))

(event Input|AxisEvents|InputAxisMoveRight
  (params (AxisValue :type Float%20%28single-precision%29))
  ;[1 1 1] Camera 2D Movement Controls
  ;;[0 0.9364 1] Camera 2D / X - Y Axis Movement
  (if (not (Variables|CameraMovement|GetDisableCameraMovement))
    (Utilities|BasicMovementControls (stale Input|AxisEvents|InputAxisMoveForward AxisValue) AxisValue) ; enters at RightMovement
  ))

(event Input|MouseEvents|MouseX
  (params (AxisValue :type Float%20%28single-precision%29))
  (if (not (Variables|CameraMovement|GetDisableCameraMovement))
    (bind (_deltaspeedx _deltaspeedy) (Utilities|EdgeScroll))
    (Transformation|AddActorLocalOffset (Variables|References|GetCameraPawnRef) (Math|Vector|MakeVector _deltaspeedx _deltaspeedy 0.0) true false)))

(event Input|MouseEvents|MouseY
  (params (AxisValue :type Float%20%28single-precision%29))
  (bind _camerapawnref (Variables|References|GetCameraPawnRef))
  (bind _returnvalue (Transformation|GetActorRotation _camerapawnref))
  ;[1 1 1] Camera Panning
  ;;[0 0.002892 1] Camera Pan X & Y
  (Utilities|FlowControl|Gate true
    (:Exit
      (Transformation|SetActorRotation _camerapawnref (Math|Rotator|MakeRotator (.roll _returnvalue) (Math|Float|Clamp(Float) (+ (.pitch _returnvalue) (* AxisValue (Variables|CameraMovement|GetPanSpeed))) -2e+01 2e+01) (.yaw _returnvalue))))))

(event Input|MouseEvents|MouseY
  (params (AxisValue :type Float%20%28single-precision%29))
  (if (not (Variables|CameraMovement|GetDisableCameraMovement))
    (Utilities|EdgeScroll) ; enters at MouseY
  ))

(event Input|MouseEvents|MouseX
  (params (AxisValue :type Float%20%28single-precision%29))
  (bind _camerapawnref (Variables|References|GetCameraPawnRef))
  (bind _returnvalue (Transformation|GetActorRotation _camerapawnref))
  ;[1 1 1] Camera Panning
  ;;[0 0.002892 1] Camera Pan X & Y
  (Utilities|FlowControl|Gate true
    (:Exit
      (Transformation|SetActorRotation _camerapawnref (Math|Rotator|MakeRotator (.roll _returnvalue) (.pitch _returnvalue) (+ (.yaw _returnvalue) (* AxisValue (Variables|CameraMovement|GetPanSpeed))))))))

(fn ConstructionScript)