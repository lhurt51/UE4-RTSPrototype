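; BP_Resource_Master is a resource actor for the RTS prototype, apparently the base for resource nodes, that sets its starting stock and look at construction.
; Its construction script optionally randomizes the resource level, then maps it to a multiplier that scales the base amount into current resources.
; Optional flags then give the mesh a random per-axis, non-uniform world scale within size limits and a random yaw.
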(fn ConstructionScript
  (bind _minmeshsize (Variables|ResourceSize|GetMinMeshSize))
  (bind _maxmeshsize (Variables|ResourceSize|GetMaxMeshSize))
  (bind _returnvalue (Math|Random|RandomFloatinRange _minmeshsize _maxmeshsize))
  (if (Variables|ResourceLegend|GetbIsRandomLevel)
    (bind _output_get (Variables|ResourceLevel|SetResourceLevel (Utilities|Enum|ByteToEnumE_ResourceLevel (Math|Conversions|ToByte(Integer) (Math|Random|RandomIntegerinRange 1 6))))))
  (switch Utilities|FlowControl|Switch|SwitchonE_ResourceLevel _output_get
    (:NewEnumerator1
      (Variables|ResourceLevel|SetResourceModifer 1.0))
    (:NewEnumerator2
      (Variables|ResourceLevel|SetResourceModifer 1.2))
    (:NewEnumerator3
      (Variables|ResourceLevel|SetResourceModifer 1.4))
    (:NewEnumerator4
      (Variables|ResourceLevel|SetResourceModifer 1.6))
    (:NewEnumerator5
      (Variables|ResourceLevel|SetResourceModifer 1.8))
    (:NewEnumerator6
      (Variables|ResourceLevel|SetResourceModifer 2.0)))
  (Variables|ResourceValue|SetCurrentResources (* (Variables|ResourceValue|GetBaseResourceAmount) (Variables|ResourceLevel|GetResourceModifer)))
  (if (Variables|ResourceLegend|GetbIsRandomSize)
    (Transformation|SetWorldScale3D (Variables|Default|GetResourceMesh) (Math|Vector|MakeVector _returnvalue _returnvalue _returnvalue)))
  (if (Variables|ResourceLegend|GetbIsRandomRotated)
    (Transformation|SetWorldRotation (Variables|Default|GetResourceMesh) (Math|Rotator|MakeRotator 0.0 0.0 (Math|Random|RandomFloatinRange 0.0 3.6e+02)) false false)))